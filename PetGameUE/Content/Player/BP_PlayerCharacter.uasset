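; Player character Blueprint that handles opening the inventory screen and playing footstep sounds.
; On BeginPlay it creates the inventory widget with a reference to itself and keeps it hidden.
; The IA_Inventory action shows the widget, switches to UI-only input and reveals the cursor; closing is not handled here.
; Tick runs the Footsteps timeline during grounded movement, whose event track plays a sand footstep sound at the character, and stops it otherwise.
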(event Input|EnhancedActionEvents|EnhancedInputActionIA_Inventory
  (params (ActionValue :type Boolean) (ElapsedSeconds :type Float%20%28double-precision%29) (TriggeredSeconds :type Float%20%28double-precision%29) (InputAction :type Input%20Action%20Object%20Reference :default "/Game/Inputs/IA_Inventory.IA_Inventory"))
  (bind _returnvalue (Game|GetPlayerController 0))
  (bind _inventoryui (Variables|Default|GetInventoryUI))
  ;[1 1 1] Inventory Open
  (Widget|SetVisibility _inventoryui "Visible")
  (Input|SetInputModeUIOnly _returnvalue _inventoryui "DoNotLock" true)
  (Variables|/Script/Engine.PlayerController|SetbShowMouseCursor _returnvalue true))

(event EventBeginPlay
  (bind _returnvalue (UserInterface|CreateWidget "/Game/UserInterface/WB_Inventory.WB_Inventory_C" (Game|GetPlayerController 0) self))
  (bind _output_get (Variables|Default|SetInventoryUI _returnvalue))
  (UserInterface|Viewport|AddtoViewport _returnvalue 0)
  (Widget|SetVisibility _output_get "Hidden"))

(event EventTick
  (params (DeltaSeconds :type Float%20%28single-precision%29))
  (if (and (> (Math|Vector|VectorLength (Transformation|GetVelocity)) 0.0) (AI|Components|NavMovement|IsMovingonGround (Pawn|GetMovementComponent)))
    (Timeline|Footsteps Play
      (:FootSteps
        (Audio|PlaySoundatLocation "/Game/Audio/Player/FootStepSand_Cue.FootStepSand_Cue" (Transformation|GetActorLocation) "0, 0, 0" 1.0 1.0 0.0 0 0 0 0)))
    (else
      (Timeline|Footsteps Stop))))

(fn ConstructionScript)